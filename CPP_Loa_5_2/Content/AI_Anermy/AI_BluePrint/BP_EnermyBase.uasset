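; Base enemy character Blueprint that handles hit reactions, with no health or death logic.
; Capsule overlap with BP_YBot sets the IsHeated hit flag, which HeatInfo exposes.
; Any damage plays a random HitMontage and nudges the enemy along the damage causer's forward vector without sweeping.
; Debug prints remain, HeatAnimation is not called here, and Wow is a stub returning false.
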(event `self.CapsuleComponent.OnComponentBeginOverlap`
  (params (OverlappedComponent :type "PrimitiveComponent Object Reference") (OtherActor :type "Actor Object Reference") (OtherComp :type "PrimitiveComponent Object Reference") (OtherBodyIndex :type Integer) (bFromSweep :type Boolean) (SweepResult :type "HitResult Structure (by ref)"))
  (`/Engine/EditorBlueprintResources/StandardMacros.IsValid` (cast `/Game/BluePrint/BP_YBot` OtherActor :!pure true)
    (:`Is Valid`
      (`KismetSystemLibrary.PrintString` "Hit!!")
      (`self.HeatEvent`))))

(event `HeatEvent`
  (set `self.IsHeated` true))

(event `HeatAnimation`
  (`|PlayMontage` null))

(event `self.ReceiveAnyDamage`
  (params (Damage :type "Float (single-precision)") (DamageType :type "DamageType Object Reference") (InstigatedBy :type "Controller Object Reference") (DamageCauser :type "Actor Object Reference"))
  (bind _hitmontage (`self.HitMontage`))
  (`KismetSystemLibrary.PrintString` "hitting")
  (set `self.Damage` DamageCauser)
  (`self.PlayAnimMontage` (`|GetArrayItem` _hitmontage (`KismetMathLibrary.RandomIntegerInRange` 0 (- (`KismetArrayLibrary.Array_Length` _hitmontage) 1))))
  (`self.K2_SetActorLocation` (+ (* (`self.GetActorForwardVector` (`self.Damage`)) 5.0) (`self.K2_GetActorLocation`))))

(fn `HeatInfo`
  (returns (IsHeat :type Boolean))
  (return (`self.IsHeated`)))

(fn `UserConstructionScript`)

(fn `wow`
  (params (NewParam :type Boolean))
  (returns (NewParam1 :type Boolean))
  (return false))