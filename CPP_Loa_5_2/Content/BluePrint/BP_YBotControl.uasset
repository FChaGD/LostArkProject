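; Player controller that moves its controlled pawn toward the mouse cursor while the right mouse button is held.
; Press and release set a flag, which Tick checks to trace under the cursor on the Visibility channel each frame.
; A hit location becomes a SimpleMoveToLocation goal only when it lies beyond a short distance from the pawn.
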(event `self.ReceiveTick`
  (params (DeltaSeconds :type "Float (single-precision)"))
  ;[0 0 0] Move Right Mouse Click
  (if true
    (if (`self.ClickRightMouse`)
      (`self.MoveToMouseCursor`))))

(event `Key|RightMouseButton`
  (params (Key :type "Key Structure"))
  ;[0 0 0] Move Right Mouse Click
  (:`Pressed`
    (`self.InputRightMousePressed`))
  (:`Released`
    (`self.InputRightMouseRelelased`)))

(fn `InputRightMousePressed`
  (set `self.ClickRightMouse` true))

(fn `InputRightMouseRelelased`
  (set `self.ClickRightMouse` false))

(fn `MoveToMouseCursor`
  (bind (_hitresult _returnvalue) (`self.GetHitResultUnderCursorByChannel` self "TraceTypeQuery1" true))
  (if _returnvalue
    (`self.SetNewDestination` (`.Location` (`GameplayStatics.BreakHitResult` _hitresult)))))

(fn `SetNewDestination`
  (params (NewDestination :type "Vector Structure"))
  (if (> (`KismetMathLibrary.Vector_Distance` NewDestination (`self.K2_GetActorLocation` (`self.K2_GetPawn`))) 60.0)
    (`AIBlueprintHelperLibrary.SimpleMoveToLocation` self NewDestination)))

(fn `UserConstructionScript`)