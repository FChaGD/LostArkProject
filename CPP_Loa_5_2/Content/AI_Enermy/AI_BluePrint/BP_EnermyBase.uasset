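; Base enemy character that initializes HP, stagger and part-destruction components from its stats on BeginPlay.
; Capsule overlap with the player (BP_YBot) triggers HeatEvent, which signals the AI controller's behavior tree and sets IsHeated, exposed through HeatInfo.
; AnyDamage only prints and stores the damage causer.
; HP subtraction, AI stopping, random hit montage and knockback logic are present but disconnected.
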(event `self.ReceiveBeginPlay`
  (bind (_hp _maxstagger _destruction) (break `/Game/AI_Enermy/Structure/EnermyStat` (`self.Stat`)))
  ;[1 1 1] 초기 스탯 설정
  (set `self.CurHP` _hp)
  (`/Game/AI_Enermy/Component/BPC_Stagger.SetDefaultStagger` (`self.BPC_Stagger`) _maxstagger)
  (`/Game/AI_Enermy/Component/BPC_PartDestruction.SetDefaultDestruction` (`self.BPC_PartDestruction`) _destruction))

(event `self.CapsuleComponent.OnComponentBeginOverlap`
  (params (OverlappedComponent :type "PrimitiveComponent Object Reference") (OtherActor :type "Actor Object Reference") (OtherComp :type "PrimitiveComponent Object Reference") (OtherBodyIndex :type Integer) (bFromSweep :type Boolean) (SweepResult :type "HitResult Structure (by ref)"))
  ;[1 1 1] 플레이어 반응
  (`/Engine/EditorBlueprintResources/StandardMacros.IsValid` (cast `/Game/Player/BP_YBot` OtherActor :!pure true)
    (:`Is Valid`
      (`self.HeatEvent`))))

(event `HeatEvent`
  ;[1 1 1] 플레이어 반응
  (message `/Game/AI_Enermy/AI_BluePrint/AI_Logic/Interface/IF_BasicAIInterface.RunBehaiverTree` (`AIBlueprintHelperLibrary.GetAIController` self))
  (set `self.IsHeated` true))

(event `HeatAnimation`
  ;[1 1 1] 플레이어 반응
  (`|PlayMontage` null))

(event `self.ReceiveAnyDamage`
  (params (Damage :type "Float (single-precision)") (DamageType :type "DamageType Object Reference") (InstigatedBy :type "Controller Object Reference") (DamageCauser :type "Actor Object Reference"))
  (`KismetSystemLibrary.PrintString` "hitting")
  (set `self.Damage` DamageCauser))

(fn `HeatInfo`
  (returns (IsHeat :type Boolean))
  (return (`self.IsHeated`)))

(fn `UserConstructionScript`)