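; Player combat component for BP_YBot that runs a seven-step punch and kick melee combo on left click.
; Each click stops movement, turns the character toward the cursor and plays the montage for ComboCount.
; Montage notifies advance the count and unlock the next attack, while a timer resets the chain.
; StartAttackTrace schedules a one-shot, debug-drawn sphere trace at the hand or foot matching ComboCount, applying BP_HPDamage on hit.
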(event `self.ReceiveBeginPlay`
  ;[1 1 1] Attack Ani
  (bind _asbp_ybot (cast `/Game/Player/BP_YBot` (`self.GetOwner`)))
  (bind _output_get (set `self.PlayerCharactor` _asbp_ybot))
  (set `self.CharatorMesh` (`Character.Mesh` _output_get)))

(event `EnhancedInput|/Game/InputSystem/입력/LeftMouseAttackClick`
  (params (ActionValue :type Boolean) (ElapsedSeconds :type "Float (double-precision)") (TriggeredSeconds :type "Float (double-precision)") (InputAction :type "InputAction Object Reference" :default "/Game/InputSystem/입력/LeftMouseAttackClick.LeftMouseAttackClick"))
  (bind _playercharactor (`self.PlayerCharactor`))
  (bind _charatormesh (`self.CharatorMesh`))
  (bind (_returnvalue_roll _returnvalue_pitch _returnvalue_yaw) (`KismetMathLibrary.BreakRotator` (`KismetMathLibrary.FindLookAtRotation` (`Actor.K2_GetActorLocation` _playercharactor) (`.Location` (`GameplayStatics.BreakHitResult` (`PlayerController.GetHitResultUnderCursorByChannel` (`GameplayStatics.GetPlayerController` 0) "TraceTypeQuery1" true))))))
  ;[1 1 1] Attack Ani
  (:`Started`
    (if (not (`self.isAttack`))
      (set `self.isAttack` true)
      (`MovementComponent.StopMovementImmediately` (`Character.CharacterMovement` _playercharactor))
      (`Actor.K2_SetActorRotation` _playercharactor (`KismetMathLibrary.MakeRotator` 0.0 0.0 _returnvalue_yaw) false)
      (switch `int` (`self.ComboCount`)
        (:`0`
          (`|PlayMontage` _charatormesh "/Game/Animation/AttackAni/Montage/YBot_SlotLeftPunch_1_Montage.YBot_SlotLeftPunch_1_Montage"
            (:`then`
              _)
            (:`OnNotifyBegin`
              (set `self.isAttack` false)
              (set `self.ComboCount` 1)))
          (`KismetSystemLibrary.K2_SetTimerDelegate` (delegate `ResetCounter`) 0.8 :!label _label))
        (:`1`
          (`|PlayMontage` _charatormesh "/Game/Animation/AttackAni/Montage/YBot_Slow2_RightPunch2_Montage.YBot_Slow2_RightPunch2_Montage"
            (:`OnNotifyBegin`
              (set `self.isAttack` false)
              (set `self.ComboCount` 2)
              (goto _label))))
        (:`2`
          (`|PlayMontage` _charatormesh "/Game/Animation/AttackAni/Montage/YBot_SlotLeftHook_3_Montage.YBot_SlotLeftHook_3_Montage"
            (:`OnNotifyBegin`
              (set `self.isAttack` false)
              (set `self.ComboCount` 3)
              (goto _label))))
        (:`3`
          (`|PlayMontage` _charatormesh "/Game/Animation/AttackAni/Montage/YBot_RightSlowPunch_4_Montage.YBot_RightSlowPunch_4_Montage"
            (:`OnNotifyBegin`
              (set `self.isAttack` false)
              (set `self.ComboCount` 4)
              (goto _label))))
        (:`4`
          (`|PlayMontage` _charatormesh "/Game/Animation/AttackAni/Montage/YBot_Left_mma_Kick5_mixamo_com_Montage.YBot_Left_mma_Kick5_mixamo_com_Montage"
            (:`OnNotifyBegin`
              (set `self.isAttack` false)
              (set `self.ComboCount` 5)
              (goto _label))))
        (:`5`
          (`|PlayMontage` _charatormesh "/Game/Animation/AttackAni/Montage/YBot_RightKick6_mixamo_com_Montage.YBot_RightKick6_mixamo_com_Montage"
            (:`OnNotifyBegin`
              (set `self.isAttack` false)
              (set `self.ComboCount` 6)
              (goto _label))))
        (:`6`
          (`|PlayMontage` _charatormesh "/Game/Animation/AttackAni/Montage/YBot_RightRotationKick7_mixamo_com_Montage.YBot_RightRotationKick7_mixamo_com_Montage"
            (:`OnNotifyBegin`
              (set `self.ComboCount` 0)
              (`KismetSystemLibrary.Delay` 0.5)
              (set `self.isAttack` false))))))))

(event `ResetCounter`
  ;[1 1 1] Attack Ani
  (set `self.ComboCount` 0))

(event `StartAttackTrace`
  ;[1 1 1] Attack Hit
  (bind _returnvalue (`KismetSystemLibrary.K2_SetTimerDelegate` (delegate `AttackTrace`) 0.01))
  (set `self.AttackTimerHandler` _returnvalue))

(event `AttackTrace`
  (bind (_start _end) (`self.GetbodyLocation` (`/Game/Player/BP_YBot.RightFoot` (`self.PlayerCharactor`))))
  (bind (_start_2 _end_2) (`self.GetbodyLocation` (`/Game/Player/BP_YBot.LeftHand` (`self.PlayerCharactor`))))
  (bind (_start_3 _end_3) (`self.GetbodyLocation` (`/Game/Player/BP_YBot.RightHand` (`self.PlayerCharactor`))))
  (bind (_start_4 _end_4) (`self.GetbodyLocation` (`/Game/Player/BP_YBot.LeftFoot` (`self.PlayerCharactor`))))
  ;[1 1 1] Attack Hit
  (switch `int` (`self.ComboCount`)
    (:`0`
      (bind (_outhit _returnvalue) (`KismetSystemLibrary.SphereTraceSingle` :`Start` _start_2 :`End` _end_2 :`Radius` 20.0 :`TraceChannel` "TraceTypeQuery1" :`DrawDebugType` "ForDuration" :`TraceColor` (struct :`A` 1.0) :!label _label_2))
      ;[1 1 1] Damage
      (if _returnvalue
        (`GameplayStatics.ApplyDamage` (`.HitActor` (`GameplayStatics.BreakHitResult` _outhit)) 30.0 null (`self.PlayerCharactor`) "/Game/Damage/BP_HPDamage.BP_HPDamage_C")))
    (:`1`
      (bind (_outhit_2 _returnvalue_2) (`KismetSystemLibrary.SphereTraceSingle` :`Start` _start_3 :`End` _end_3 :`Radius` 20.0 :`TraceChannel` "TraceTypeQuery1" :`DrawDebugType` "ForDuration" :!label _label_3))
      (if _returnvalue_2
        (`GameplayStatics.ApplyDamage` (`.HitActor` (`GameplayStatics.BreakHitResult` _outhit_2)) 30.0 null (`self.PlayerCharactor`) "/Game/Damage/BP_HPDamage.BP_HPDamage_C")))
    (:`2`
      (goto _label_2))
    (:`3`
      (goto _label_3))
    (:`4`
      (bind (_outhit_3 _returnvalue_3) (`KismetSystemLibrary.SphereTraceSingle` :`Start` _start_4 :`End` _end_4 :`Radius` 20.0 :`TraceChannel` "TraceTypeQuery1" :`DrawDebugType` "ForDuration"))
      (if _returnvalue_3
        (`GameplayStatics.ApplyDamage` (`.HitActor` (`GameplayStatics.BreakHitResult` _outhit_3)) 30.0 null (`self.PlayerCharactor`) "/Game/Damage/BP_HPDamage.BP_HPDamage_C")))
    (:`5`
      (bind (_outhit_4 _returnvalue_4) (`KismetSystemLibrary.SphereTraceSingle` :`Start` _start :`End` _end :`Radius` 20.0 :`TraceChannel` "TraceTypeQuery1" :`DrawDebugType` "ForDuration" :`TraceColor` (struct :`G` 0.044537 :`B` 1.0 :`A` 1.0) :!label _label_4))
      (if _returnvalue_4
        (`GameplayStatics.ApplyDamage` (`.HitActor` (`GameplayStatics.BreakHitResult` _outhit_4)) 30.0 null (`self.PlayerCharactor`) "/Game/Damage/BP_HPDamage.BP_HPDamage_C")))
    (:`6`
      (goto _label_4))))

(event `StopAttackTrace`
  ;[1 1 1] Attack Hit
  (`KismetSystemLibrary.K2_ClearAndInvalidateTimerHandle` (`self.AttackTimerHandler`)))

(fn `GetbodyLocation`
  (params (self2 :type "SceneComponent Object Reference"))
  (returns (Start :type "Vector Structure") (End :type "Vector Structure"))
  (return (`SceneComponent.K2_GetComponentLocation` self2) (`KismetMathLibrary.TransformLocation` (`SceneComponent.K2_GetComponentToWorld` self2) (+ (`SceneComponent.RelativeLocation` self2) (20.0 0.0 0.0)))))